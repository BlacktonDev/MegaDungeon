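; Player character for a puzzle-style game where queued directional inputs play out as grid-like hops on execute.
; Input events fill ActionArray, which IA_Execute dispatches and clears, while Tick wipes it beyond six entries.
; Each move turns the mesh, then repeats line trace, jump, location step and delay until blocked.
; It also pins the camera to BP_CamPos, adds the arrows widget, counts bonus bones and identifies itself as the player.
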(event Custom|MoveCamera
  ;[1 1 1] FixedCamera
  (bind _returnvalue (Actor|GetActorOfClass "/Game/_Romo/Character/BP_CamPos.BP_CamPos_C"))
  (Transformation|AttachComponentToComponent (Variables|Default|GetCamera) (Variables|/Game/_Romo/Character/BP_CamPos.BP_CamPos_C|GetArrow _returnvalue) "None" "KeepRelative" "KeepRelative" "KeepRelative" true))

(event Custom|MoveUp
  (bind _returnvalue (Transformation|GetActorLocation))
  (bind _returnvalue_2 (Transformation|GetActorLocation))
  (Transformation|SetWorldRotation (Variables|Character|GetMesh) "0.000000,-90.000000,0.000000" false false)
  (for _index (range 0 0) :!label _label
    (Utilities|FlowControl|DoOnce false
      (:Completed
        (bind _outhit (Collision|LineTraceByChannel (Transformation|GetActorLocation) (Math|Vector|MakeVector (+ (.x _returnvalue_2) (Variables|Default|GetDistanceToComprobe)) (.y _returnvalue_2) (.z _returnvalue_2)) "TraceTypeQuery1" false 0 "ForOneFrame"))
        (if (.bBlockingHit (Collision|BreakHitResult _outhit))
          (Development|PrintString "camino bloqueado")
          (Variables|Default|SetCanMove? true)
          (else
            (Character|Jump)
            (Transformation|SetActorLocation (Math|Vector|MakeVector (+ (.x _returnvalue) (Variables|Default|GetDistanceToMove)) (.y _returnvalue) (.z _returnvalue)) false false)
            (Utilities|FlowControl|Delay (Variables|Default|GetJumpTime))
            (Character|StopJumping)
            (goto _label))))))
  (Utilities|FlowControl|DoOnce false) ; enters at Reset
)

(event Custom|MoveDown
  (bind _returnvalue (Transformation|GetActorLocation))
  (bind _returnvalue_2 (Transformation|GetActorLocation))
  (Transformation|SetWorldRotation (Variables|Character|GetMesh) "0.000000,90.000000,0.000000" false false)
  (for _index (range 0 0) :!label _label
    (Utilities|FlowControl|DoOnce false
      (:Completed
        (bind _outhit (Collision|LineTraceByChannel (Transformation|GetActorLocation) (Math|Vector|MakeVector (- (.x _returnvalue_2) (Variables|Default|GetDistanceToComprobe)) (.y _returnvalue_2) (.z _returnvalue_2)) "TraceTypeQuery1" false 0 "ForOneFrame"))
        (if (.bBlockingHit (Collision|BreakHitResult _outhit))
          (Development|PrintString "camino bloqueado")
          (Variables|Default|SetCanMove? true)
          (else
            (Character|Jump)
            (Transformation|SetActorLocation (Math|Vector|MakeVector (- (.x _returnvalue) (Variables|Default|GetDistanceToMove)) (.y _returnvalue) (.z _returnvalue)) false false)
            (Utilities|FlowControl|Delay (Variables|Default|GetJumpTime))
            (Character|StopJumping)
            (goto _label))))))
  (Utilities|FlowControl|DoOnce false) ; enters at Reset
)

(event Custom|MoveRight
  (bind _returnvalue (Transformation|GetActorLocation))
  (bind _returnvalue_2 (Transformation|GetActorLocation))
  (Transformation|SetWorldRotation (Variables|Character|GetMesh) "0, 0, 0" false false)
  (for _index (range 0 0) :!label _label
    (Utilities|FlowControl|DoOnce false
      (:Completed
        (bind _outhit (Collision|LineTraceByChannel (Transformation|GetActorLocation) (Math|Vector|MakeVector (.x _returnvalue_2) (+ (.y _returnvalue_2) (Variables|Default|GetDistanceToComprobe)) (.z _returnvalue_2)) "TraceTypeQuery1" false 0 "ForOneFrame"))
        (if (.bBlockingHit (Collision|BreakHitResult _outhit))
          (Development|PrintString "camino bloqueado")
          (Variables|Default|SetCanMove? true)
          (else
            (Character|Jump)
            (Transformation|SetActorLocation (Math|Vector|MakeVector (.x _returnvalue) (+ (.y _returnvalue) (Variables|Default|GetDistanceToMove)) (.z _returnvalue)) false false)
            (Utilities|FlowControl|Delay (Variables|Default|GetJumpTime))
            (Character|StopJumping)
            (goto _label))))))
  (Utilities|FlowControl|DoOnce false) ; enters at Reset
)

(event Custom|MoveLeft
  (bind _returnvalue (Transformation|GetActorRotation))
  (bind _returnvalue_2 (Transformation|GetActorLocation))
  (bind _returnvalue_3 (Transformation|GetActorLocation))
  (Transformation|SetWorldRotation (Variables|Character|GetMesh) "0.000000,180.000000,0.000000" false false)
  (Transformation|SetActorRotation (Math|Rotator|MakeRotator (.roll _returnvalue) (.pitch _returnvalue) -9e+01))
  (for _index (range 0 0) :!label _label
    (Utilities|FlowControl|DoOnce false
      (:Completed
        (bind _outhit (Collision|LineTraceByChannel (Transformation|GetActorLocation) (Math|Vector|MakeVector (.x _returnvalue_3) (- (.y _returnvalue_3) (Variables|Default|GetDistanceToComprobe)) (.z _returnvalue_3)) "TraceTypeQuery1" false 0 "ForOneFrame"))
        (if (.bBlockingHit (Collision|BreakHitResult _outhit))
          (Development|PrintString "camino bloqueado")
          (Variables|Default|SetCanMove? true)
          (else
            (Character|Jump)
            (Transformation|SetActorLocation (Math|Vector|MakeVector (.x _returnvalue_2) (- (.y _returnvalue_2) (Variables|Default|GetDistanceToMove)) (.z _returnvalue_2)) false false)
            (Utilities|FlowControl|Delay (Variables|Default|GetJumpTime))
            (Character|StopJumping)
            (goto _label))))))
  (Utilities|FlowControl|DoOnce false) ; enters at Reset
)

(event Input|EnhancedActionEvents|EnhancedInputActionIA_MoveUp
  (params (ActionValue :type Boolean) (ElapsedSeconds :type Float%20%28double-precision%29) (TriggeredSeconds :type Float%20%28double-precision%29) (InputAction :type Input%20Action%20Object%20Reference :default "/Game/_Romo/Character/Input/IA_MoveUp.IA_MoveUp"))
  (:Completed
    (bind _output_get (Variables|Default|SetActionString "Up"))
    (Utilities|Array|Add (Variables|Default|GetActionArray) _output_get)))

(event Input|EnhancedActionEvents|EnhancedInputActionIA_MoveDown
  (params (ActionValue :type Boolean) (ElapsedSeconds :type Float%20%28double-precision%29) (TriggeredSeconds :type Float%20%28double-precision%29) (InputAction :type Input%20Action%20Object%20Reference :default "/Game/_Romo/Character/Input/IA_MoveDown.IA_MoveDown"))
  (:Completed
    (bind _output_get (Variables|Default|SetActionString "Down"))
    (Utilities|Array|Add (Variables|Default|GetActionArray) _output_get)))

(event Input|EnhancedActionEvents|EnhancedInputActionIA_MoveLeft
  (params (ActionValue :type Boolean) (ElapsedSeconds :type Float%20%28double-precision%29) (TriggeredSeconds :type Float%20%28double-precision%29) (InputAction :type Input%20Action%20Object%20Reference :default "/Game/_Romo/Character/Input/IA_MoveLeft.IA_MoveLeft"))
  (:Completed
    (bind _output_get (Variables|Default|SetActionString "Left"))
    (Utilities|Array|Add (Variables|Default|GetActionArray) _output_get)))

(event Input|EnhancedActionEvents|EnhancedInputActionIA_MoveRight
  (params (ActionValue :type Boolean) (ElapsedSeconds :type Float%20%28double-precision%29) (TriggeredSeconds :type Float%20%28double-precision%29) (InputAction :type Input%20Action%20Object%20Reference :default "/Game/_Romo/Character/Input/IA_MoveRight.IA_MoveRight"))
  (:Completed
    (bind _output_get (Variables|Default|SetActionString "Right"))
    (Utilities|Array|Add (Variables|Default|GetActionArray) _output_get)))

(event Input|EnhancedActionEvents|EnhancedInputActionIA_Execute
  (params (ActionValue :type Boolean) (ElapsedSeconds :type Float%20%28double-precision%29) (TriggeredSeconds :type Float%20%28double-precision%29) (InputAction :type Input%20Action%20Object%20Reference :default "/Game/_Romo/Character/Input/IA_Execute.IA_Execute"))
  (:Completed
    (if (Variables|Default|GetCanMove?)
      (for _array_element (Variables|Default|GetActionArray)
        (switch string _array_element
          (:Up
            (CallFunction|MoveUp))
          (:Down
            (CallFunction|MoveDown))
          (:Left
            (CallFunction|MoveLeft))
          (:Right
            (CallFunction|MoveRight))))
      (Utilities|Array|Clear (Variables|Default|GetActionArray)))))

(event EventBeginPlay
  (bind _returnvalue (Game|GetPlayerState 0))
  (bind _returnvalue_2 (Game|GetPlayerController _returnvalue))
  ;[1 1 1] Input
  (bind _asplayer_controller (Utilities|Casting|CastToPlayerController (Pawn|GetController)))
  (Utilities|IsValid (PlayerController|LocalPlayerSubsystems|GetEnhancedInputLocalPlayerSubsystem _asplayer_controller)
    (:Is%20Valid
      (Input|AddMappingContext (PlayerController|LocalPlayerSubsystems|GetEnhancedInputLocalPlayerSubsystem _asplayer_controller) "/Game/_Romo/Character/Input/IMC_RomoInput.IMC_RomoInput" 0 "(bIgnoreAllPressedKeysUntilRelease=True,bForceImmediately=False,bNotifyUserSettings=False)")
      (CallFunction|MoveCamera)
      (Variables|/Script/Engine.PlayerController|SetbShowMouseCursor _returnvalue_2 true)
      (bind _returnvalue_3 (UserInterface|CreateWidget "/Game/_Romo/Character/WB_Arrows.WB_Arrows_C" _returnvalue_2))
      (UserInterface|Viewport|AddtoViewport _returnvalue_3 0))))

(event EventTick
  (params (DeltaSeconds :type Float%20%28single-precision%29))
  (if (not (>= 6 (Utilities|Array|Length (Variables|Default|GetActionArray))))
    (Utilities|Array|Clear (Variables|Default|GetActionArray))))

(fn ConstructionScript)

(fn AddBonusBone
  (bind _result (Math|Integer|IncrementInt (Variables|Default|GetboneCount))
    (:%20%20
      (Development|PrintString (Utilities|String|Append "Numero de wesos: " (Utilities|String|ToString(Integer) (Math|Integer|Clamp(Integer) _result 0 3)))))))

(fn CheckIsPlayer
  (return true self))