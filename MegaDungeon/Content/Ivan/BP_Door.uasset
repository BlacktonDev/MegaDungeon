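; Locked door actor that slides open once when a player carrying a key enters its trigger box.
; On overlap, it identifies the player through a CheckIsPlayerMessage call on the other actor and reads HasKey.
; With a key, it disables the trigger's collision and a Timeline offsets the Cube from its cached starting relative location.
; Without one, it prints a Spanish missing-key message.
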(event OnComponentBeginOverlap(Box)
  (params (OverlappedComponent :type Primitive%20Component%20Object%20Reference) (OtherActor :type Actor%20Object%20Reference) (OtherComp :type Primitive%20Component%20Object%20Reference) (OtherBodyIndex :type Integer) (bFromSweep :type Boolean) (SweepResult :type Hit%20Result%20Structure%20%28by%20ref%29))
  (bind (_isplayer _playeractor) (Class|BPIPlayer|CheckIsPlayer(Message) OtherActor))
  (if _isplayer
    (if (Variables|/Game/_Romo/Character/BP_MDCharacter.BP_MDCharacter_C|GethasKey _playeractor)
      (Collision|SetCollisionEnabled (Variables|Default|GetBox) "NoCollision")
      (bind _newtrack_0 (Timeline|Timeline Play)
        (:Update
          (Transformation|SetRelativeLocation (Variables|Default|GetCube) (+ (Variables|Default|GetinitialLocation) _newtrack_0) false false)))
      (else
        (Development|PrintString "Falta llave")))))

(event EventBeginPlay
  (Variables|Default|SetinitialLocation (Variables|/Script/Engine.SceneComponent|GetRelativeLocation (Variables|Default|GetCube))))

(fn ConstructionScript)