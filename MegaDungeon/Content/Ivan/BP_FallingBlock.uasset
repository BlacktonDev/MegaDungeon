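; BP_FallingBlock is a block that gives way once the player leaves it, exposing a deadly hazard.
; When the player's overlap with FallTrigger ends, it hides that trigger and the Cylinder, then enables DeathTrigger and the Cone, which start disabled.
; A player overlapping DeathTrigger reloads the current level.
; The fall is a visibility and trigger-collision swap with no movement, and players are identified through a CheckIsPlayerMessage call.
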(event OnComponentBeginOverlap(DeathTrigger)
  (params (OverlappedComponent :type Primitive%20Component%20Object%20Reference) (OtherActor :type Actor%20Object%20Reference) (OtherComp :type Primitive%20Component%20Object%20Reference) (OtherBodyIndex :type Integer) (bFromSweep :type Boolean) (SweepResult :type Hit%20Result%20Structure%20%28by%20ref%29))
  (bind _isplayer (Class|BPIPlayer|CheckIsPlayer(Message) OtherActor))
  (if _isplayer
    (bind _returnvalue (Game|GetCurrentLevelName true))
    (Game|OpenLevel(byName) (Utilities|String|StringToName _returnvalue))))

(event OnComponentEndOverlap(FallTrigger)
  (params (OverlappedComponent :type Primitive%20Component%20Object%20Reference) (OtherActor :type Actor%20Object%20Reference) (OtherComp :type Primitive%20Component%20Object%20Reference) (OtherBodyIndex :type Integer))
  (bind _isplayer (Class|BPIPlayer|CheckIsPlayer(Message) OtherActor))
  (if _isplayer
    (CallFunction|FlipDeathComponents true)
    (CallFunction|FlipFallComponents false)
    (Development|PrintString "Salido")))

(event EventBeginPlay
  (CallFunction|FlipDeathComponents false))

(fn ConstructionScript)

(fn FlipDeathComponents
  (params (isActive :type Boolean))
  (bind _deathtrigger (Variables|Default|GetDeathTrigger))
  (Rendering|SetVisibility _deathtrigger isActive false)
  (if isActive
    (Collision|SetCollisionEnabled _deathtrigger "QueryAndPhysics")
    (else
      (Collision|SetCollisionEnabled _deathtrigger "NoCollision")))
  (Rendering|SetVisibility (Variables|Default|GetCone) isActive false))

(fn FlipFallComponents
  (params (isActive :type Boolean))
  (bind _falltrigger (Variables|Default|GetFallTrigger))
  (Rendering|SetVisibility _falltrigger isActive false)
  (if isActive
    (Collision|SetCollisionEnabled _falltrigger "QueryAndPhysics")
    (else
      (Collision|SetCollisionEnabled _falltrigger "NoCollision")))
  (Rendering|SetVisibility (Variables|Default|GetCylinder) isActive true))