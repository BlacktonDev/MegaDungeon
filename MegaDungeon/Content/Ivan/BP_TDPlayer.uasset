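; BP_TDPlayer is a player Blueprint that counts bonus bones and identifies itself as the player.
; BoneCount resets to zero on BeginPlay, and AddBonusBone increments it, then prints a debug message with the value clamped to a small range for display only, leaving the stored count uncapped.
; CheckIsPlayer returns true along with a self reference, letting callers confirm and obtain the player actor.
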(event EventBeginPlay
  (Variables|Default|SetboneCount 0))

(fn ConstructionScript)

(fn AddBonusBone
  (bind _result (Math|Integer|IncrementInt (Variables|Default|GetboneCount))
    (:%20%20
      (Development|PrintString (Utilities|String|Append "Numero de wesos: " (Utilities|String|ToString(Integer) (Math|Integer|Clamp(Integer) _result 0 3)))))))

(fn CheckIsPlayer
  (return true self))